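; BP_PawnTank is the player tank pawn's Blueprint, handling HUD updates and XP-based leveling.
; Tick pushes health, XP and level to the game mode's in-game HUD, updates the reload widget component, then polls OnLevelUp.
; When XP reaches its maximum, it raises the level, carries over surplus XP and recalculates the threshold.
; OnPowerUp then opens the upgrade widget, pauses the game and immediately recalculates damage and fire rate.
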(event `self.ReceiveBeginPlay`
  ;[1 1 1] Begin Play
  (bind _asbp_tank_game_mode_base (cast `/Game/Blueprints/GameModes/BP_TankGameModeBase` (`GameplayStatics.GetGameMode`)))
  (set `self.BP Tank Game Mode Base` _asbp_tank_game_mode_base))

(event `self.ReceiveTick`
  (params (DeltaSeconds :type "Float (single-precision)"))
  ;[1 1 1] Update Display Widget
  (message `/Game/Blueprints/Interfaces/BPI_ToonTanks.UpdateHealthBar` (`/Game/Blueprints/GameModes/BP_TankGameModeBase.WBP_InGameHUD` (`self.BP Tank Game Mode Base`)) (`self.GetHealthBarValue`))
  (message `/Game/Blueprints/Interfaces/BPI_ToonTanks.UpdateXPBar` (`/Game/Blueprints/GameModes/BP_TankGameModeBase.WBP_InGameHUD` (`self.BP Tank Game Mode Base`)) (`KismetMathLibrary.SafeDivide` (`self.CurrentExperience`) (`self.MaxExperience`)))
  (`/Game/Blueprints/Interfaces/BPI_ToonTanks.UpdateLevel` (`/Game/Blueprints/GameModes/BP_TankGameModeBase.WBP_InGameHUD` (`self.BP Tank Game Mode Base`)) (`self.PlayerLevel`))
  (message `/Game/Blueprints/Interfaces/BPI_ToonTanks.UpdateReloadBar` (`WidgetComponent.GetUserWidgetObject` (`self.ReloadWidgetComponent`)) (`self.GetReloadBarValue`))
  (`self.OnLevelUp`))

(event `OnLevelUp`
  ;[1 1 1] Update XP Bar and Player Level
  (if (>= (`self.CurrentExperience`) (`self.MaxExperience`))
    (`/Engine/EditorBlueprintResources/StandardMacros.IncrementInt` (`self.PlayerLevel`)
      (:`  `
        (set `self.CurrentExperience` (- (`self.CurrentExperience`) (`self.MaxExperience`)))
        (bind _returnvalue (`self.CalculateMaxExperience` (`self.PlayerLevel`)))
        (set `self.MaxExperience` _returnvalue)
        (`self.OnPowerUp`)))))

(fn `OnPowerUp`
  ;[1 1 1] Call Upgrade Widget
  (bind _returnvalue (`|CreateWidget` "/Game/Blueprints/Widgets/Components/WBP_UpgradeOption.WBP_UpgradeOption_C"))
  (`UserWidget.AddToViewport` _returnvalue 0)
  (`GameplayStatics.SetGamePaused` true)
  ;[1 1 1] Recalculate Damage and Fire Rate
  (bind _returnvalue_2 (`self.CalculateDamage` (`self.PowerLevel`)))
  (set `self.Damage` _returnvalue_2)
  (bind _returnvalue_3 (`self.CalculateFireRate` (`self.AttackSpeedLevel`)))
  (set `self.FireRate` _returnvalue_3))

(fn `UserConstructionScript`)