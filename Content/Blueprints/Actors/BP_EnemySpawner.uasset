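; Enemy spawner that adds enemy tanks at random reachable navmesh points around the player tank while it is alive.
; A looping timer drives spawning, capped by a max count checked against the enemy list that Tick refreshes every frame.
; A second timer periodically raises the cap and lowers SpawnInterval, though the running spawn timer is never reset with the new value.
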(event `self.ReceiveBeginPlay`
  (`KismetSystemLibrary.K2_SetTimerDelegate` (`|CreateDelegate` :!event `SpawnEnemies`) (`self.SpawnInterval`) true)
  (bind _returnvalue (`GameplayStatics.GetActorOfClass` "/Game/Blueprints/Pawns/BP_PawnTank.BP_PawnTank_C"))
  (set `self.PlayerPawn` _returnvalue)
  (`KismetSystemLibrary.K2_SetTimerDelegate` (delegate `IncreaseMaxEnemy`) 45.0 true))

(event `IncreaseMaxEnemy`
  (bind _result (`/Engine/EditorBlueprintResources/StandardMacros.IncrementInt` (`self.MaxEnemyCount`))
    (:`  `
      (set `self.MaxEnemyCount` _result)
      (set `self.SpawnInterval` (- (`self.SpawnInterval`) 0.05)))))

(event `self.ReceiveTick`
  (params (DeltaSeconds :type "Float (single-precision)"))
  (bind _outactors (`GameplayStatics.GetAllActorsOfClass` "/Game/Blueprints/Pawns/BP_PawnEnemyTank.BP_PawnEnemyTank_C"))
  (set `self.Enemy` _outactors))

(event `SpawnEnemies`
  (if (and (`PawnTank.bIsPlayerAlive` (`self.PlayerPawn`)) (< (`KismetArrayLibrary.Array_Length` (`self.Enemy`)) (`self.MaxEnemyCount`)))
    (`|SpawnActorFromClass` "/Game/Blueprints/Pawns/BP_PawnEnemyTank.BP_PawnEnemyTank_C" (`KismetMathLibrary.MakeTransform` (`KismetMathLibrary.MakeVector` (.x (`NavigationSystemV1.K2_GetRandomReachablePointInRadius` (`self.K2_GetActorLocation` (`self.PlayerPawn`)) 1400.0 null null)) (.y (`NavigationSystemV1.K2_GetRandomReachablePointInRadius` (`self.K2_GetActorLocation` (`self.PlayerPawn`)) 1400.0 null null)) (+ (.z (`NavigationSystemV1.K2_GetRandomReachablePointInRadius` (`self.K2_GetActorLocation` (`self.PlayerPawn`)) 1400.0 null null)) 60.0))) "AdjustIfPossibleButDontSpawnIfColliding" "OverrideRootScale" null null)))

(fn `UserConstructionScript`)