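; Player controller for the tank game that handles pausing and the game-over screen.
; On BeginPlay it disables input until the game mode's StartDelay elapses.
; G or Escape toggles PauseGame, which pauses the game and adds or removes WBP_PauseMenu.
; EndGame pauses, then after a delay reuses WBP_PauseMenu for the result and high score, switches to UI-only input and stops the pawn's tick.
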(event `self.ReceiveBeginPlay`
  (bind (_asbp_tank_game_mode_base _bsuccess) (cast `/Game/Blueprints/GameModes/BP_TankGameModeBase` (`GameplayStatics.GetGameMode`) :!pure true))
  (bind _asbp_tank_game_mode_base_2 (cast `/Game/Blueprints/GameModes/BP_TankGameModeBase` (`GameplayStatics.GetGameMode`)))
  (set `self.As BP Tank Game Mode Base` _asbp_tank_game_mode_base_2)
  ;[1 1 1] Enable Pause Input after Start Delay is over
  (`self.DisableInput` null)
  (if _bsuccess
    (`KismetSystemLibrary.Delay` (`KismetMathLibrary.Conv_IntToDouble` (`TankGameModeBase.StartDelay` _asbp_tank_game_mode_base)))
    (`self.EnableInput` null)))

(event `Key|G`
  (params (Key :type "Key Structure"))
  (:`Pressed`
    (`self.PauseGame` :!label _label)))

(event `Key|Escape`
  (params (Key :type "Key Structure"))
  (:`Pressed`
    (goto _label)))

(event `EndGame`
  (params (bPaused :type Boolean) (NewHiScore :type Boolean) (HiScore :type Integer))
  ;[1 1 1] Game Over
  (`GameplayStatics.SetGamePaused` true)
  (`KismetSystemLibrary.Delay` 1.0)
  (bind _returnvalue (`|CreateWidget` "/Game/Blueprints/Widgets/WBP_PauseMenu.WBP_PauseMenu_C"))
  (`/Game/Blueprints/Widgets/WBP_PauseMenu.OnEndGame` _returnvalue bPaused NewHiScore HiScore)
  (`UserWidget.AddToViewport` _returnvalue 0)
  (`WidgetBlueprintLibrary.SetInputMode_UIOnlyEx` self null "LockInFullscreen")
  (set `self.bShowMouseCursor` true)
  (`self.SetActorTickEnabled` (`GameplayStatics.GetPlayerPawn` 0) false))

(fn `PauseGame`
  (if (not (`self.IsPaused`))
    (bind _output_get (set `self.IsPaused` true))
    (`GameplayStatics.SetGamePaused` _output_get)
    (bind _returnvalue (`|CreateWidget` "/Game/Blueprints/Widgets/WBP_PauseMenu.WBP_PauseMenu_C" self))
    (bind _output_get_2 (set `self.WBP_PauseMenu` _returnvalue))
    (`UserWidget.AddToViewport` _output_get_2 0)
    (`/Game/Blueprints/Widgets/WBP_PauseMenu.OnPauseGame` (`self.WBP_PauseMenu`) (`self.IsPaused`))
    (else
      (bind _output_get_3 (set `self.IsPaused` false))
      (`GameplayStatics.SetGamePaused` _output_get_3)
      (`Widget.RemoveFromParent` (`self.WBP_PauseMenu`)))))

(fn `UserConstructionScript`)