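; Base game mode for the tank game that runs match start, HUD updates, game over and return to the main menu.
; GameStart looks up the current level in DT_Level, creates the in-game HUD and, in survival mode, spawns the enemy spawner after a delay.
; GameOver saves GameScore to the BP_ScoreSave slot if it is a new high score, then passes the result to the player controller.
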(event `self.GameStart`
  ;[1 1 1] Start Game
  (`WidgetBlueprintLibrary.SetInputMode_GameOnly` (`GameplayStatics.GetPlayerController` 0))
  (`GameplayStatics.SetViewportMouseCaptureMode` "CapturePermanently_IncludingInitialMouseDown")
  (bind _returnvalue (`GameplayStatics.GetCurrentLevelName` true))
  (bind _returnvalue_2 (`|GetDataTableRow` "/Game/DataTable/DT_Level.DT_Level" (`KismetStringLibrary.Conv_StringToName` _returnvalue))
    (:`then`
      (set `self.bIsSurvivalMode` (`.IsSurvival_2_8C9C6172486DC314F312A798C95FEBAC` (break `/Game/DataTable/TankStructure` _returnvalue_2)))
      (`self.CreateDisplayWidget`)
      ;[1 1 1] Create Spawner Actor
      (if (`self.bIsSurvivalMode`)
        (`KismetSystemLibrary.Delay` (+ (`KismetMathLibrary.Conv_IntToDouble` (`self.StartDelay`)) 1.5))
        (`|SpawnActorFromClass` "/Game/Blueprints/Actors/BP_EnemySpawner.BP_EnemySpawner_C" (`KismetMathLibrary.MakeTransform` (0.0 0.0 30.0)) "Undefined" "OverrideRootScale" null null)))))

(event `CreateDisplayWidget`
  ;[1 1 1] Create Widget
  (bind _returnvalue (`|CreateWidget` "/Game/Blueprints/Widgets/WBP_InGameHUD.WBP_InGameHUD_C"))
  (bind _output_get (set `self.WBP_InGameHUD` _returnvalue))
  (set `/Game/Blueprints/Widgets/WBP_InGameHUD.SurvivalMode` (`self.bIsSurvivalMode`) (`self.WBP_InGameHUD`))
  (`/Game/Blueprints/Widgets/WBP_InGameHUD.Set Start Count Down` _output_get (`self.StartDelay`))
  (message `/Game/Blueprints/Interfaces/BPI_ToonTanks.UpdateGameTime` (`self.WBP_InGameHUD`) (`self.GameMinutes`) (`self.GameSeconds`))
  (`self.SetHighScore`)
  (`UserWidget.AddToViewport` (`self.WBP_InGameHUD`) 0))

(event `SetHighScore`
  ;[1 1 1] High Score
  (bind _returnvalue (`GameplayStatics.LoadGameFromSlot` "BP_ScoreSave"))
  (bind _asbp_score_save (cast `/Game/DataTable/BP_ScoreSave` _returnvalue))
  (message `/Game/Blueprints/Interfaces/BPI_ToonTanks.UpdateHighScore` (`self.WBP_InGameHUD`) (`/Game/DataTable/BP_ScoreSave.PlayerScore` _asbp_score_save)))

(event `self.DisplayGameTimer`
  (params (Minutes :type Integer) (Seconds :type Integer))
  ;[1 1 1] Display Timer
  (message `/Game/Blueprints/Interfaces/BPI_ToonTanks.UpdateGameTime` (`self.WBP_InGameHUD`) Minutes Seconds))

(event `self.DisplayScore`
  (params (Score :type Integer))
  ;[1 1 1] Display Score
  (`/Game/Blueprints/Widgets/WBP_InGameHUD.WidgetDisplayScore` (`self.WBP_InGameHUD`) Score))

(event `self.GameOver`
  (params (PlayerWon :type Boolean))
  ;[1 1 1] End Game
  (`/Game/Blueprints/Interfaces/BPI_ToonTanks.UpdateHealthBar` (`self.WBP_InGameHUD`) 0.0)
  (bind _asbp_player_controller (cast `/Game/Blueprints/PlayerControllers/BP_PlayerController` (`GameplayStatics.GetPlayerController` 0)))
  (`self.CreateScoreBoard`)
  (`/Game/Blueprints/PlayerControllers/BP_PlayerController.EndGame` _asbp_player_controller PlayerWon (`self.NewHiScore`) (`/Game/DataTable/BP_ScoreSave.PlayerScore` (`self.ScoreSave`))))

(event `CreateScoreBoard`
  ;[1 1 1] High Score
  (bind _returnvalue (`GameplayStatics.DoesSaveGameExist` "BP_ScoreSave"))
  (if _returnvalue
    (`/Engine/EditorBlueprintResources/StandardMacros.DoOnce` false
      (:`Completed`
        (bind _returnvalue_2 (`GameplayStatics.LoadGameFromSlot` "BP_ScoreSave"))
        (bind _asbp_score_save (cast `/Game/DataTable/BP_ScoreSave` _returnvalue_2))
        (bind _output_get (set `self.ScoreSave` _asbp_score_save))
        (if (< (`/Game/DataTable/BP_ScoreSave.PlayerScore` _output_get) (`self.GameScore`))
          (set `/Game/DataTable/BP_ScoreSave.PlayerScore` (`self.GameScore`) (`self.ScoreSave`) :!label _label)
          (bind _returnvalue_3 (`GameplayStatics.SaveGameToSlot` (`self.ScoreSave`) "BP_ScoreSave"))
          (set `self.NewHiScore` _returnvalue_3))))
    (else
      (bind _returnvalue_4 (`GameplayStatics.CreateSaveGameObject` "/Game/DataTable/BP_ScoreSave.BP_ScoreSave_C"))
      (set `self.ScoreSave` _returnvalue_4)
      (goto _label))))

(fn `QuitGame`
  (`GameplayStatics.OpenLevel` "MainMenu"))

(fn `UserConstructionScript`)